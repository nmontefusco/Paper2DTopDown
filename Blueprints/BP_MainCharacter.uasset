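; Player knight character with Paper2D flipbook animation, eight-way input movement and a cycling four-swing attack.
; Tick applies normalized input movement, remembers the last direction, and sets the flipbook returned by UpdateAnimation.
; UpdateAnimation branches on current or last axis signs to pick four-direction idle, walk or attack sprites.
; Attack press advances the swing counter and locks movement for a short delay; releasing clears the attack flag early.
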(event `self.ReceiveTick`
  (params (DeltaSeconds :type "Float (single-precision)"))
  (`|ExecutionSequence`
    (:`then_0`
      (if (or (!= (`self.GetInputAxisValue`) 0.0) (!= (`self.GetInputAxisValue`) 0.0))
        (set `self.LastRightValue` (`self.GetInputAxisValue`))
        (set `self.LastUpValue` (`self.GetInputAxisValue`))
        (`self.AddMovementInput` (`KismetMathLibrary.Normal` (`KismetMathLibrary.MakeVector` (`self.GetInputAxisValue`) (`self.GetInputAxisValue`))))))
    (:`then_1`
      (bind _currentanimation (`self.UpdateAnimation` (`self.GetInputAxisValue`) (* (`self.GetInputAxisValue`) -1.0) (`self.LastRightValue`) (* (`self.LastUpValue`) -1.0)))
      (`PaperFlipbookComponent.SetFlipbook` _currentanimation))))

(event `InputAction|Attack`
  (params (Key :type "Key Structure"))
  (bind _numswings (`self.numSwings`))
  (:`Pressed`
    (if (not (`self.is_attacking`))
      (set `self.is_attacking` true)
      (`CharacterMovementComponent.DisableMovement` (`self.CharacterMovement`))
      (bind _result (`/Engine/EditorBlueprintResources/StandardMacros.IncrementInt` _numswings)
        (:`  `
          (set `self.numSwings` _result)
          (if (== _numswings 4)
            (set `self.numSwings` 0))
          (`KismetSystemLibrary.Delay` 0.4)
          (set `self.is_attacking` false)
          (`CharacterMovementComponent.SetMovementMode` (`self.CharacterMovement`) "MOVE_Walking" 0)))))
  (:`Released`
    (set `self.is_attacking` false)))

(fn `UpdateAnimation`
  (params (RightAxis :type "Float (double-precision)") (UpAxis :type "Float (double-precision)") (LastRight :type "Float (double-precision)") (lastUp :type "Float (double-precision)"))
  (returns (CurrentAnimation :type "PaperFlipbook Object Reference"))
  (locals (RightLocal :type "Float (double-precision)") (UpLocal :type "Float (double-precision)") (AnimationLocal :type "PaperFlipbook Object Reference") (LastRightLocal :type "Float (double-precision)") (LastUpLocal :type "Float (double-precision)"))
  (set `local.RightLocal` RightAxis)
  (set `local.UpLocal` UpAxis)
  (set `local.LastRightLocal` LastRight)
  (set `local.LastUpLocal` lastUp)
  (`/Engine/EditorBlueprintResources/StandardMacros.CompareFloat` (`local.RightLocal`)
    (:`>`
      (`/Engine/EditorBlueprintResources/StandardMacros.CompareFloat` (`local.UpLocal`)
        (:`>`
          (if (`self.is_attacking`)
            (switch `int` (`self.numSwings`)
              (:`Default`
                (set `local.AnimationLocal` "/Game/FlipBooks/sprKnight_Up_Attack_1_strip6.sprKnight_Up_Attack_1_strip6" :!label _label))
              (:`0`
                (goto _label))
              (:`1`
                (set `local.AnimationLocal` "/Game/FlipBooks/sprKnight_Up_Attack_2_strip6.sprKnight_Up_Attack_2_strip6"))
              (:`2`
                (set `local.AnimationLocal` "/Game/FlipBooks/sprKnight_Up_Attack_3_strip6.sprKnight_Up_Attack_3_strip6"))
              (:`3`
                (set `local.AnimationLocal` "/Game/FlipBooks/sprKnight_Up_Attack_4_strip8.sprKnight_Up_Attack_4_strip8")))
            (else
              (set `local.AnimationLocal` "/Game/FlipBooks/Up/sprKnight_Up_Walk_strip6.sprKnight_Up_Walk_strip6"))))
        (:`==`
          (if (`self.is_attacking`)
            (switch `int` (`self.numSwings`)
              (:`Default`
                (set `local.AnimationLocal` "/Game/FlipBooks/Right/sprKnight_Right_Attack_1_strip6.sprKnight_Right_Attack_1_strip6" :!label _label_2))
              (:`0`
                (goto _label_2))
              (:`1`
                (set `local.AnimationLocal` "/Game/FlipBooks/Right/sprKnight_Right_Attack_2_strip6.sprKnight_Right_Attack_2_strip6"))
              (:`2`
                (set `local.AnimationLocal` "/Game/FlipBooks/Right/sprKnight_Right_Attack_3_strip6.sprKnight_Right_Attack_3_strip6"))
              (:`3`
                (set `local.AnimationLocal` "/Game/FlipBooks/Right/sprKnight_Right_Attack_4_strip9.sprKnight_Right_Attack_4_strip9")))
            (else
              (set `local.AnimationLocal` "/Game/FlipBooks/Right/sprKnight_Right_Walk_strip6.sprKnight_Right_Walk_strip6"))))
        (:`<`
          (if (`self.is_attacking`)
            (switch `int` (`self.numSwings`)
              (:`Default`
                (set `local.AnimationLocal` "/Game/FlipBooks/Right/sprKnight_Right_Attack_1_strip6.sprKnight_Right_Attack_1_strip6" :!label _label_3))
              (:`0`
                (goto _label_3))
              (:`1`
                (set `local.AnimationLocal` "/Game/FlipBooks/Right/sprKnight_Right_Attack_2_strip6.sprKnight_Right_Attack_2_strip6"))
              (:`2`
                (set `local.AnimationLocal` "/Game/FlipBooks/Right/sprKnight_Right_Attack_3_strip6.sprKnight_Right_Attack_3_strip6"))
              (:`3`
                (set `local.AnimationLocal` "/Game/FlipBooks/Right/sprKnight_Right_Attack_4_strip9.sprKnight_Right_Attack_4_strip9")))
            (else
              (set `local.AnimationLocal` "/Game/FlipBooks/Right/sprKnight_Right_Walk_strip6.sprKnight_Right_Walk_strip6"))))))
    (:`==`
      (`/Engine/EditorBlueprintResources/StandardMacros.CompareFloat` (`local.UpLocal`)
        (:`>`
          (if (`self.is_attacking`)
            (switch `int` (`self.numSwings`)
              (:`Default`
                (set `local.AnimationLocal` "/Game/FlipBooks/sprKnight_Up_Attack_1_strip6.sprKnight_Up_Attack_1_strip6" :!label _label_4))
              (:`0`
                (goto _label_4))
              (:`1`
                (set `local.AnimationLocal` "/Game/FlipBooks/sprKnight_Up_Attack_2_strip6.sprKnight_Up_Attack_2_strip6"))
              (:`2`
                (set `local.AnimationLocal` "/Game/FlipBooks/sprKnight_Up_Attack_3_strip6.sprKnight_Up_Attack_3_strip6"))
              (:`3`
                (set `local.AnimationLocal` "/Game/FlipBooks/sprKnight_Up_Attack_4_strip8.sprKnight_Up_Attack_4_strip8")))
            (else
              (set `local.AnimationLocal` "/Game/FlipBooks/Up/sprKnight_Up_Walk_strip6.sprKnight_Up_Walk_strip6"))))
        (:`==`
          (`/Engine/EditorBlueprintResources/StandardMacros.CompareFloat` (`local.LastRightLocal`)
            (:`>`
              (`/Engine/EditorBlueprintResources/StandardMacros.CompareFloat` (`local.LastUpLocal`)
                (:`>`
                  (if (`self.is_attacking`)
                    (switch `int` (`self.numSwings`)
                      (:`Default`
                        (set `local.AnimationLocal` "/Game/FlipBooks/Right/sprKnight_Right_Attack_1_strip6.sprKnight_Right_Attack_1_strip6" :!label _label_5))
                      (:`0`
                        (goto _label_5))
                      (:`1`
                        (set `local.AnimationLocal` "/Game/FlipBooks/Right/sprKnight_Right_Attack_2_strip6.sprKnight_Right_Attack_2_strip6"))
                      (:`2`
                        (set `local.AnimationLocal` "/Game/FlipBooks/Right/sprKnight_Right_Attack_3_strip6.sprKnight_Right_Attack_3_strip6"))
                      (:`3`
                        (set `local.AnimationLocal` "/Game/FlipBooks/Right/sprKnight_Right_Attack_4_strip9.sprKnight_Right_Attack_4_strip9")))
                    (else
                      (set `local.AnimationLocal` "/Game/FlipBooks/Right/sprKnight_Right_Idle_strip5.sprKnight_Right_Idle_strip5"))))
                (:`==`
                  (if (`self.is_attacking`)
                    (switch `int` (`self.numSwings`)
                      (:`Default`
                        (set `local.AnimationLocal` "/Game/FlipBooks/Right/sprKnight_Right_Attack_1_strip6.sprKnight_Right_Attack_1_strip6" :!label _label_6))
                      (:`0`
                        (goto _label_6))
                      (:`1`
                        (set `local.AnimationLocal` "/Game/FlipBooks/Right/sprKnight_Right_Attack_2_strip6.sprKnight_Right_Attack_2_strip6"))
                      (:`2`
                        (set `local.AnimationLocal` "/Game/FlipBooks/Right/sprKnight_Right_Attack_3_strip6.sprKnight_Right_Attack_3_strip6"))
                      (:`3`
                        (set `local.AnimationLocal` "/Game/FlipBooks/Right/sprKnight_Right_Attack_4_strip9.sprKnight_Right_Attack_4_strip9")))
                    (else
                      (set `local.AnimationLocal` "/Game/FlipBooks/Right/sprKnight_Right_Idle_strip5.sprKnight_Right_Idle_strip5"))))
                (:`<`
                  (if (`self.is_attacking`)
                    (switch `int` (`self.numSwings`)
                      (:`Default`
                        (set `local.AnimationLocal` "/Game/FlipBooks/Right/sprKnight_Right_Attack_1_strip6.sprKnight_Right_Attack_1_strip6" :!label _label_7))
                      (:`0`
                        (goto _label_7))
                      (:`1`
                        (set `local.AnimationLocal` "/Game/FlipBooks/Right/sprKnight_Right_Attack_2_strip6.sprKnight_Right_Attack_2_strip6"))
                      (:`2`
                        (set `local.AnimationLocal` "/Game/FlipBooks/Right/sprKnight_Right_Attack_3_strip6.sprKnight_Right_Attack_3_strip6"))
                      (:`3`
                        (set `local.AnimationLocal` "/Game/FlipBooks/Right/sprKnight_Right_Attack_4_strip9.sprKnight_Right_Attack_4_strip9")))
                    (else
                      (set `local.AnimationLocal` "/Game/FlipBooks/Right/sprKnight_Right_Idle_strip5.sprKnight_Right_Idle_strip5"))))))
            (:`==`
              (`/Engine/EditorBlueprintResources/StandardMacros.CompareFloat` (`local.LastUpLocal`)
                (:`>`
                  (if (`self.is_attacking`)
                    (switch `int` (`self.numSwings`)
                      (:`Default`
                        (set `local.AnimationLocal` "/Game/FlipBooks/sprKnight_Up_Attack_1_strip6.sprKnight_Up_Attack_1_strip6" :!label _label_8))
                      (:`0`
                        (goto _label_8))
                      (:`1`
                        (set `local.AnimationLocal` "/Game/FlipBooks/sprKnight_Up_Attack_2_strip6.sprKnight_Up_Attack_2_strip6"))
                      (:`2`
                        (set `local.AnimationLocal` "/Game/FlipBooks/sprKnight_Up_Attack_3_strip6.sprKnight_Up_Attack_3_strip6"))
                      (:`3`
                        (set `local.AnimationLocal` "/Game/FlipBooks/sprKnight_Up_Attack_4_strip8.sprKnight_Up_Attack_4_strip8")))
                    (else
                      (set `local.AnimationLocal` "/Game/FlipBooks/Up/sprKnight_Up_Idle_strip5.sprKnight_Up_Idle_strip5"))))
                (:`==`
                  (if (`self.is_attacking`)
                    (switch `int` (`self.numSwings`)
                      (:`Default`
                        (set `local.AnimationLocal` "/Game/FlipBooks/Down/sprKnight_Down_Attack_1_strip6.sprKnight_Down_Attack_1_strip6" :!label _label_9))
                      (:`0`
                        (goto _label_9))
                      (:`1`
                        (set `local.AnimationLocal` "/Game/FlipBooks/Down/sprKnight_Down_Attack_2_strip6.sprKnight_Down_Attack_2_strip6"))
                      (:`2`
                        (set `local.AnimationLocal` "/Game/FlipBooks/Down/sprKnight_Down_Attack_3_strip6.sprKnight_Down_Attack_3_strip6"))
                      (:`3`
                        (set `local.AnimationLocal` "/Game/FlipBooks/Down/sprKnight_Down_Attack_4_strip8.sprKnight_Down_Attack_4_strip8")))
                    (else
                      ;[1 1 1] This is Start Animation
                      (set `local.AnimationLocal` "/Game/FlipBooks/Down/sprKnight_Down_Idle_strip5.sprKnight_Down_Idle_strip5"))))
                (:`<`
                  (if (`self.is_attacking`)
                    (switch `int` (`self.numSwings`)
                      (:`Default`
                        (set `local.AnimationLocal` "/Game/FlipBooks/Down/sprKnight_Down_Attack_1_strip6.sprKnight_Down_Attack_1_strip6" :!label _label_10))
                      (:`0`
                        (goto _label_10))
                      (:`1`
                        (set `local.AnimationLocal` "/Game/FlipBooks/Down/sprKnight_Down_Attack_2_strip6.sprKnight_Down_Attack_2_strip6"))
                      (:`2`
                        (set `local.AnimationLocal` "/Game/FlipBooks/Down/sprKnight_Down_Attack_3_strip6.sprKnight_Down_Attack_3_strip6"))
                      (:`3`
                        (set `local.AnimationLocal` "/Game/FlipBooks/Down/sprKnight_Down_Attack_4_strip8.sprKnight_Down_Attack_4_strip8")))
                    (else
                      (set `local.AnimationLocal` "/Game/FlipBooks/Down/sprKnight_Down_Idle_strip5.sprKnight_Down_Idle_strip5"))))))
            (:`<`
              (`/Engine/EditorBlueprintResources/StandardMacros.CompareFloat` (`local.LastUpLocal`)
                (:`>`
                  (if (`self.is_attacking`)
                    (switch `int` (`self.numSwings`)
                      (:`Default`
                        (set `local.AnimationLocal` "/Game/FlipBooks/Left/sprKnight_Left_Attack_1_strip6.sprKnight_Left_Attack_1_strip6" :!label _label_11))
                      (:`0`
                        (goto _label_11))
                      (:`1`
                        (set `local.AnimationLocal` "/Game/FlipBooks/Left/sprKnight_Left_Attack_2_strip6.sprKnight_Left_Attack_2_strip6"))
                      (:`2`
                        (set `local.AnimationLocal` "/Game/FlipBooks/Left/sprKnight_Left_Attack_3_strip6.sprKnight_Left_Attack_3_strip6"))
                      (:`3`
                        (set `local.AnimationLocal` "/Game/FlipBooks/Left/sprKnight_Left_Attack_4_strip9.sprKnight_Left_Attack_4_strip9")))
                    (else
                      (set `local.AnimationLocal` "/Game/FlipBooks/Left/sprKnight_Left_Idle_strip5.sprKnight_Left_Idle_strip5"))))
                (:`==`
                  (if (`self.is_attacking`)
                    (switch `int` (`self.numSwings`)
                      (:`Default`
                        (set `local.AnimationLocal` "/Game/FlipBooks/Left/sprKnight_Left_Attack_1_strip6.sprKnight_Left_Attack_1_strip6" :!label _label_12))
                      (:`0`
                        (goto _label_12))
                      (:`1`
                        (set `local.AnimationLocal` "/Game/FlipBooks/Left/sprKnight_Left_Attack_2_strip6.sprKnight_Left_Attack_2_strip6"))
                      (:`2`
                        (set `local.AnimationLocal` "/Game/FlipBooks/Left/sprKnight_Left_Attack_3_strip6.sprKnight_Left_Attack_3_strip6"))
                      (:`3`
                        (set `local.AnimationLocal` "/Game/FlipBooks/Left/sprKnight_Left_Attack_4_strip9.sprKnight_Left_Attack_4_strip9")))
                    (else
                      (set `local.AnimationLocal` "/Game/FlipBooks/Left/sprKnight_Left_Idle_strip5.sprKnight_Left_Idle_strip5"))))
                (:`<`
                  (if (`self.is_attacking`)
                    (switch `int` (`self.numSwings`)
                      (:`Default`
                        (set `local.AnimationLocal` "/Game/FlipBooks/Down/sprKnight_Down_Attack_1_strip6.sprKnight_Down_Attack_1_strip6" :!label _label_13))
                      (:`0`
                        (goto _label_13))
                      (:`1`
                        (set `local.AnimationLocal` "/Game/FlipBooks/Down/sprKnight_Down_Attack_2_strip6.sprKnight_Down_Attack_2_strip6"))
                      (:`2`
                        (set `local.AnimationLocal` "/Game/FlipBooks/Down/sprKnight_Down_Attack_3_strip6.sprKnight_Down_Attack_3_strip6"))
                      (:`3`
                        (set `local.AnimationLocal` "/Game/FlipBooks/Down/sprKnight_Down_Attack_4_strip8.sprKnight_Down_Attack_4_strip8")))
                    (else
                      (set `local.AnimationLocal` "/Game/FlipBooks/Down/sprKnight_Down_Idle_strip5.sprKnight_Down_Idle_strip5"))))))))
        (:`<`
          (if (`self.is_attacking`)
            (switch `int` (`self.numSwings`)
              (:`Default`
                (set `local.AnimationLocal` "/Game/FlipBooks/Down/sprKnight_Down_Attack_1_strip6.sprKnight_Down_Attack_1_strip6" :!label _label_14))
              (:`0`
                (goto _label_14))
              (:`1`
                (set `local.AnimationLocal` "/Game/FlipBooks/Down/sprKnight_Down_Attack_2_strip6.sprKnight_Down_Attack_2_strip6"))
              (:`2`
                (set `local.AnimationLocal` "/Game/FlipBooks/Down/sprKnight_Down_Attack_3_strip6.sprKnight_Down_Attack_3_strip6"))
              (:`3`
                (set `local.AnimationLocal` "/Game/FlipBooks/Down/sprKnight_Down_Attack_4_strip8.sprKnight_Down_Attack_4_strip8")))
            (else
              (set `local.AnimationLocal` "/Game/FlipBooks/Down/sprKnight_Down_Walk_strip6.sprKnight_Down_Walk_strip6"))))))
    (:`<`
      (`/Engine/EditorBlueprintResources/StandardMacros.CompareFloat` (`local.UpLocal`)
        (:`>`
          (if (`self.is_attacking`)
            (switch `int` (`self.numSwings`)
              (:`Default`
                (set `local.AnimationLocal` "/Game/FlipBooks/Left/sprKnight_Left_Attack_1_strip6.sprKnight_Left_Attack_1_strip6" :!label _label_15))
              (:`0`
                (goto _label_15))
              (:`1`
                (set `local.AnimationLocal` "/Game/FlipBooks/Left/sprKnight_Left_Attack_2_strip6.sprKnight_Left_Attack_2_strip6"))
              (:`2`
                (set `local.AnimationLocal` "/Game/FlipBooks/Left/sprKnight_Left_Attack_3_strip6.sprKnight_Left_Attack_3_strip6"))
              (:`3`
                (set `local.AnimationLocal` "/Game/FlipBooks/Left/sprKnight_Left_Attack_4_strip9.sprKnight_Left_Attack_4_strip9")))
            (else
              (set `local.AnimationLocal` "/Game/FlipBooks/Left/sprKnight_Left_Walk_strip6.sprKnight_Left_Walk_strip6"))))
        (:`==`
          (if (`self.is_attacking`)
            (switch `int` (`self.numSwings`)
              (:`Default`
                (set `local.AnimationLocal` "/Game/FlipBooks/Left/sprKnight_Left_Attack_1_strip6.sprKnight_Left_Attack_1_strip6" :!label _label_16))
              (:`0`
                (goto _label_16))
              (:`1`
                (set `local.AnimationLocal` "/Game/FlipBooks/Left/sprKnight_Left_Attack_2_strip6.sprKnight_Left_Attack_2_strip6"))
              (:`2`
                (set `local.AnimationLocal` "/Game/FlipBooks/Left/sprKnight_Left_Attack_3_strip6.sprKnight_Left_Attack_3_strip6"))
              (:`3`
                (set `local.AnimationLocal` "/Game/FlipBooks/Left/sprKnight_Left_Attack_4_strip9.sprKnight_Left_Attack_4_strip9")))
            (else
              (set `local.AnimationLocal` "/Game/FlipBooks/Left/sprKnight_Left_Walk_strip6.sprKnight_Left_Walk_strip6"))))
        (:`<`
          (if (`self.is_attacking`)
            (switch `int` (`self.numSwings`)
              (:`Default`
                (set `local.AnimationLocal` "/Game/FlipBooks/Down/sprKnight_Down_Attack_1_strip6.sprKnight_Down_Attack_1_strip6" :!label _label_17))
              (:`0`
                (goto _label_17))
              (:`1`
                (set `local.AnimationLocal` "/Game/FlipBooks/Down/sprKnight_Down_Attack_2_strip6.sprKnight_Down_Attack_2_strip6"))
              (:`2`
                (set `local.AnimationLocal` "/Game/FlipBooks/Down/sprKnight_Down_Attack_3_strip6.sprKnight_Down_Attack_3_strip6"))
              (:`3`
                (set `local.AnimationLocal` "/Game/FlipBooks/Down/sprKnight_Down_Attack_4_strip8.sprKnight_Down_Attack_4_strip8")))
            (else
              (set `local.AnimationLocal` "/Game/FlipBooks/Down/sprKnight_Down_Walk_strip6.sprKnight_Down_Walk_strip6")))))))
  (return (`local.AnimationLocal`)))

(fn `UserConstructionScript`)